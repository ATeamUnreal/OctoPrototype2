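; BP_LobbyPC is the lobby player controller that sets up lobby UI and starts travel to the Game map.
; Without a head-mounted display, BeginPlay shows a lobby widget and mouse cursor on authority and creates a collapsed loading widget regardless of authority.
; GameStart has authority call ShowLoading on every BP_LobbyPC to reveal that widget.
; A separate sequence branch, outside the authority check, runs servertravel after a short delay.
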(event Custom|GameStart
  (Utilities|FlowControl|Sequence
    (:then_0
      (Networking|SwitchHasAuthority
        (:Authority
          (bind _outactors (Actor|GetAllActorsOfClass "BP_LobbyPC_C"))
          (for _array_element _outactors
            (CallFunction|ShowLoading _array_element)))))
    (:then_1
      (Utilities|FlowControl|Delay 2.0)
      (Development|ExecuteConsoleCommand "servertravel/Game/Maps/Game" 0))))

(event Custom|ShowLoading
  (bind _lobbyloadingwidget (Variables|Default|GetLobbyLoadingWidget))
  (Utilities|IsValid _lobbyloadingwidget
    (:Is%20Valid
      (Widget|SetVisibility _lobbyloadingwidget "Visible"))))

(event EventBeginPlay
  (if (not (Class|HeadMountedDisplayFunctionLibrary|IsHeadMountedDisplayEnabled))
    (Utilities|FlowControl|Sequence
      (:then_0
        (Networking|SwitchHasAuthority
          (:Authority
            (bind _returnvalue (UserInterface|CreateWidget "/Game/Blueprints/Lobby/LobbyWidget.LobbyWidget_C"))
            (UserInterface|Viewport|AddtoViewport _returnvalue 0)
            (Variables|Default|SetbShowMouseCursor true))))
      (:then_1
        (bind _returnvalue_2 (UserInterface|CreateWidget "/Game/Blueprints/Lobby/LobbyLoadingWidget.LobbyLoadingWidget_C"))
        (UserInterface|Viewport|AddtoViewport _returnvalue_2 0)
        (bind _output_get (Variables|Default|SetLobbyLoadingWidget _returnvalue_2))
        (Widget|SetVisibility _output_get "Collapsed")))))

(event EventTick
  (params (DeltaSeconds :type Float%20%28single-precision%29)))

(fn ConstructionScript)