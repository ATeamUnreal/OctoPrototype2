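; Lobby game mode that spawns and possesses a pawn for each player as they log in.
; On PostLogin it caches the level's PlayerStart actors, spawns at the one matching the running player index, then increments the index.
; The first player gets the VR pawn if a headset is enabled where the game mode runs; other slots get the PC pawn.
; A pawn-shrinking branch and per-slot transform selection are left unused.
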(event EventPostLogin
  (params (NewPlayer :type Player%20Controller%20Object%20Reference))
  (bind _pcplayer (Variables|Default|GetpcPlayer))
  (CallFunction|GetStartPos)
  (bind _returnvalue (Game|SpawnActorfromClass (Utilities|Select :Index (Variables|Default|GetPlayerIndex) :Option%200 (select (Class|HeadMountedDisplayFunctionLibrary|IsHeadMountedDisplayEnabled) "/Game/Blueprints/Octopus/BP_VRPawnMain.BP_VRPawnMain_C" _pcplayer) :Option%201 _pcplayer :Option%202 _pcplayer :Option%203 _pcplayer :Option%204 _pcplayer) (Transformation|GetActorTransform (Utilities|Array|Get(acopy) (Variables|Default|GetPlayerLocations) (Variables|Default|GetPlayerIndex))) "AlwaysSpawn" 0 0))
  (bind _aspawn (Utilities|Casting|CastToPawn _returnvalue))
  (Utilities|IsValid _aspawn
    (:Is%20Valid
      (Pawn|Possess NewPlayer _aspawn)
      (Math|Integer|IncrementInt (Variables|Default|GetPlayerIndex)))))

(fn ConstructionScript)

(fn GetStartPos
  (if (== (Utilities|Array|Length (Variables|Default|GetPlayerLocations)) 0)
    (bind _outactors (Actor|GetAllActorsOfClass "/Script/Engine.PlayerStart"))
    (Variables|Default|SetPlayerLocations _outactors)))