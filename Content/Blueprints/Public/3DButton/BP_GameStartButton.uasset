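; BP_GameStartButton is a 3D lobby button, built from two BP_Letter child actors, that starts the game.
; Highlight lights both letters, while HighlightBack calls itself after the first letter cast rather than that letter's HighlightBack.
; The first motion controller overlap with its box, given a valid game mode, latches IsClicked and calls ClickServer on both letters.
; After a short delay it calls GameStart on player 0's BP_LobbyPC.
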(event OnComponentBeginOverlap(Box)
  (params (OverlappedComponent :type Primitive%20Component%20Object%20Reference) (OtherActor :type Actor%20Object%20Reference) (OtherComp :type Primitive%20Component%20Object%20Reference) (OtherBodyIndex :type Integer) (bFromSweep :type Boolean) (SweepResult :type Hit%20Result%20Structure%20%28by%20ref%29))
  (if (not (Variables|Default|GetIsClicked))
    (Utilities|Casting|CastToBP_MotionControllerMain OtherActor)
    (Utilities|IsValid (Game|GetGameMode)
      (:Is%20Valid
        (Variables|Default|SetIsClicked true)
        (Utilities|FlowControl|Sequence
          (:then_0
            (bind _asbp_letter (Utilities|Casting|CastToBP_Letter (Variables|/Script/Engine.ChildActorComponent|GetChildActor (Variables|Default|GetChildActor))))
            (Default|ClickServer _asbp_letter))
          (:then_1
            (bind _asbp_letter_2 (Utilities|Casting|CastToBP_Letter (Variables|/Script/Engine.ChildActorComponent|GetChildActor (Variables|Default|GetChildActor1))))
            (Default|ClickServer _asbp_letter_2))
          (:then_2
            (Utilities|FlowControl|Delay 1.0)
            (bind _asbp_lobby_pc (Utilities|Casting|CastToBP_LobbyPC (Game|GetPlayerController 0)))
            (Default|GameStart _asbp_lobby_pc)))))))

(event EventHighlight
  (bind _asbp_letter (Utilities|Casting|CastToBP_Letter (Variables|/Script/Engine.ChildActorComponent|GetChildActor (Variables|Default|GetChildActor))))
  (Default|Highlight _asbp_letter)
  (bind _asbp_letter_2 (Utilities|Casting|CastToBP_Letter (Variables|/Script/Engine.ChildActorComponent|GetChildActor (Variables|Default|GetChildActor1))))
  (Default|Highlight _asbp_letter_2))

(event EventHighlightBack
  (Utilities|Casting|CastToBP_Letter (Variables|/Script/Engine.ChildActorComponent|GetChildActor (Variables|Default|GetChildActor)))
  (CallFunction|HighlightBack)
  (bind _asbp_letter (Utilities|Casting|CastToBP_Letter (Variables|/Script/Engine.ChildActorComponent|GetChildActor (Variables|Default|GetChildActor1))))
  (Default|HighlightBack _asbp_letter))

(fn ConstructionScript)