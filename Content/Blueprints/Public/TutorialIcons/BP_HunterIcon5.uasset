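; BP_HunterIcon5 is a tutorial icon for non-VR (hunter) players that reveals a text widget when its trigger box is overlapped.
; On BeginPlay it hides the widget, then either hides the icon and disables collision for a VR pawn, or sets the text and default color.
; The first overlap shows the widget, switches to the selected color and plays a click sound.
; Color enums map to a scalar material parameter.
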(event OnComponentBeginOverlap(Box)
  (params (OverlappedComponent :type Primitive%20Component%20Object%20Reference) (OtherActor :type Actor%20Object%20Reference) (OtherComp :type Primitive%20Component%20Object%20Reference) (OtherBodyIndex :type Integer) (bFromSweep :type Boolean) (SweepResult :type Hit%20Result%20Structure%20%28by%20ref%29))
  ;[1 1 1] 겹쳐지면 텍스트 띄우기
  (if (not (Variables|Default|GetActivated))
    (Variables|Default|SetActivated true)
    (Rendering|SetVisibility (Variables|Default|GetWidget) true false)
    (Rendering|Material|SetScalarParameterValueonMaterials (Variables|Default|GetIcon) "Color" (Utilities|Select :Index (Variables|Default|GetSelectedColor) :NewEnumerator0 0.01 :NewEnumerator1 0.1 :NewEnumerator2 0.2 :NewEnumerator3 0.3 :NewEnumerator4 0.4 :NewEnumerator10 0.5 :NewEnumerator5 0.6 :NewEnumerator6 0.7 :NewEnumerator9 1.0))
    (Audio|SpawnSoundatLocation "/Game/Ultimate_SFX_Bundle/Casual_Bundle/UI_Item_Sounds/Cues/8_Bit_click_sounds/8_Bit_click_sounds_7_Cue.8_Bit_click_sounds_7_Cue" (Transformation|GetWorldLocation (Variables|Default|GetIcon)) "0, 0, 0" 1.0 1.0 0.0 0 0)))

(event EventBeginPlay
  ;[1 1 1] 로컬 플레이어가 vr이면 아이콘을 숨기고, 헌터면 텍스트 설정
  (Rendering|SetVisibility (Variables|Default|GetWidget) false false)
  (Utilities|Casting|CastToBP_VRPawnMain (Pawn|GetControlledPawn (Game|GetPlayerController 0))
    (:then
      (Rendering|SetVisibility (Variables|Default|GetIcon) false false)
      (Collision|SetCollisionEnabled (Variables|Default|GetBox) "NoCollision"))
    (:CastFailed
      (bind _aspctutorial_text (Utilities|Casting|CastToPCTutorialText (UserInterface|GetUserWidgetObject (Variables|Default|GetWidget))))
      (Default|SetText _aspctutorial_text (Variables|Default|GetText))
      (Rendering|Material|SetScalarParameterValueonMaterials (Variables|Default|GetIcon) "Color" (Utilities|Select :Index (Variables|Default|GetDefaultColor) :NewEnumerator0 0.01 :NewEnumerator1 0.1 :NewEnumerator2 0.2 :NewEnumerator3 0.3 :NewEnumerator4 0.4 :NewEnumerator10 0.5 :NewEnumerator5 0.6 :NewEnumerator6 0.7 :NewEnumerator9 1.0)))))

(fn ConstructionScript)