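; Game instance for a VR octopus versus hunters multiplayer game, holding match state, player role, skins and UID slots.
; Role picks the VR or TPS start map and offsets skin lookup for an octopus host.
; Session events host a listen-server Lobby, join the first found session (ignoring the IP), and server-travel between Lobby and Main.
; Starting a match destroys the session and copies lobby UID slots for Main; network errors reset state to Ready.
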(event Custom|ReadyForGame
  ;[1 1 1] 맵이동
  ;;[1 1 1] EntryMap에서 분기
  (bind _isoctopus (CallFunction|IsOctopus))
  (if _isoctopus
    (Game|OpenLevel(byName) "VRStart")
    (else
      (Game|OpenLevel(byName) "TPSStart"))))

(event Custom|Debug%20Show%20Collision
  ;[1 0.6443 0] Debug
  (Development|ExecuteConsoleCommand "Show Collision" 0))

(event Custom|OpenLobby_Listen
  ;[1 1 1] 맵이동
  ;;[1 1 1] Lobby 리슨 서버로 열기
  (|Session (Game|GetPlayerController 0) 5 false
    (:OnSuccess
      (Development|PrintString "Create session!" true true "(R=0.021359,G=1.000000,B=0.000000,A=1.000000)" 15.0)
      (Game|OpenLevel(byName) "Lobby" true "listen"))
    (:OnFailure
      ;;[1 1 1] 에러처리 고민
      (Development|PrintString "Failed to create session" true true "(R=1.000000,G=0.452495,B=0.000000,A=1.000000)" 15.0))))

(event Custom|ConnectToListenServer
  (params (IP :type Name))
  (bind _returnvalue (Game|GetPlayerController 0))
  ;[1 1 1] 맵이동
  ;;[1 1 1] 리슨 서버에 IP입력하여 연결
  (bind _results (|FindSessions _returnvalue 5 false)
    (:OnSuccess
      (Development|PrintString (Utilities|String|Append "Search Succees : count : " (Utilities|String|ToString(Integer) (Utilities|Array|Length _results))) true true "(R=0.021359,G=1.000000,B=0.000000,A=1.000000)" 15.0)
      (if (> (Utilities|Array|Length _results) 0)
        (|JoinSession _returnvalue (Utilities|Array|Get(acopy) _results)
          (:OnSuccess
            (Development|PrintString "Join Seuccess" true true "(R=0.021359,G=1.000000,B=0.000000,A=1.000000)" 15.0))
          (:OnFailure
            (Development|PrintString "Failed to join session" true true "(R=1.000000,G=0.452495,B=0.000000,A=1.000000)" 15.0)))))))

(event Custom|BackToLobby
  ;[1 1 1] 맵이동
  (Utilities|FlowControl|Delay 1.0)
  (CallFunction|SetState "Ready")
  (|Session (Game|GetPlayerController 0) 5 false
    (:OnSuccess
      (Development|PrintString "Create session!" true true "(R=0.021359,G=1.000000,B=0.000000,A=1.000000)" 15.0)
      (Development|ExecuteConsoleCommand "servertravel/Game/Maps/Lobby" 0))))

(event Custom|StartMainGame
  (params (DelayTime :type Float%20%28single-precision%29))
  ;[1 1 1] 맵이동
  (|DestroySession (Game|GetPlayerController 0)
    (:OnSuccess
      (Development|PrintString "Destroy Session!" true true "(R=0.021359,G=1.000000,B=0.000000,A=1.000000)" 15.0)
      (CallFunction|SetState "StartGame")
      (CallFunction|CopyHasUIDList)
      (Utilities|FlowControl|Delay DelayTime)
      (Development|ExecuteConsoleCommand "servertravel/Game/Maps/Main" 0))))

(event EventHandleNetworkError
  (params (FailureType :type ENetworkFailure%20Enum :default "NetDriverAlreadyExists") (bIsServer :type Boolean))
  (CallFunction|SetState "Ready")
  (Development|PrintString (Utilities|String|EnumtoString FailureType) true true "(R=0.000000,G=0.660000,B=1.000000,A=1.000000)" 1e+01)
  (Development|PrintString (Utilities|String|ToString(Boolean) bIsServer) true true "(R=1.000000,G=0.087969,B=0.000000,A=1.000000)" 1e+01))

(event EventInit
  ;[1 1 1] Init
  (CallFunction|SetHasUIDList)
  (CallFunction|SetState "Ready")
  (Skin|SetSkinList))

(fn SetGIRoleState
  (params (State :type ERoleState%20Enum :default "NewEnumerator0"))
  (Variables|Default|SetGI_RoleState State))

(fn IsOctopus
  (return (Utilities|Enum|Equal(Enum) (Variables|Default|GetGI_RoleState) "NewEnumerator0")))

(fn GetSkin
  (params (Index :type Integer))
  (bind _returnvalue (- Index 1))
  ;[1 1 1] 서버가 Octo일 때는 헌터플레이어 인덱스는 1부터 시작하니 빼준다
  (bind _isoctopus (CallFunction|IsOctopus))
  (if _isoctopus
    (if (>= _returnvalue 0)
      (return (Utilities|Array|Get(acopy) (Variables|Skin|GetSkins) _returnvalue)))
    (else
      (return (Utilities|Array|Get(acopy) (Variables|Skin|GetSkins) Index)))))

(fn SortSkinList
  (bind _skins (Variables|Skin|GetSkins))
  (bind _skins_2 (Variables|Skin|GetSkins))
  (bind _returnvalue (Utilities|Array|Length _skins_2))
  (for _index (range 0 (* (Utilities|Array|Length (Variables|Skin|GetSkins)) 3))
    (LocalVariables|SetIndex1 (Math|Random|RandomInteger _returnvalue))
    (LocalVariables|SetIndex2 (Math|Random|RandomInteger _returnvalue))
    (bind _output_get (LocalVariables|SetTemp (Utilities|Array|Get(acopy) _skins (LocalVariables|GetIndex1))))
    (Utilities|Array|SetArrayElem (Variables|Skin|GetSkins) (LocalVariables|GetIndex1) (Utilities|Array|Get(acopy) _skins (LocalVariables|GetIndex2)))
    (Utilities|Array|SetArrayElem (Variables|Skin|GetSkins) (LocalVariables|GetIndex2) _output_get)))

(fn SetSkinList
  (for _index (range 0 (- (|GetNumEnumEntries) 1))
    (Utilities|Array|Add (Variables|Skin|GetSkins) (Utilities|Enum|ByteToEnumESkinState (Math|Conversions|ToByte(Integer) _index)))))

(fn SetLocalUID
  (params (NewUID :type Integer))
  (Variables|Default|SetLocalUID NewUID))

(fn SetLocalSkinState
  (params (SkinState :type ESkinState%20Enum :default "NewEnumerator0"))
  (Variables|Skin|SetLocalSkinState SkinState))

(fn SetState
  (params (State :type EGameState%20Enum :default "Ready"))
  (Variables|Default|SetCurrentState State))

(fn SetHasUIDList
  (for _index (range 0 (Variables|Default|GetMaxPlayerCount))
    (Utilities|Array|Add (Variables|Default|GetHasUIDList) false)))

(fn GetUID
  (bind _hasuidlist (Variables|Default|GetHasUIDList))
  (for (_array_element _array_index) _hasuidlist
    (if (not _array_element)
      (Utilities|Array|SetArrayElem _hasuidlist _array_index true)
      (return _array_index))))

(fn SetUIDEmpty
  (params (UID :type Integer))
  (Utilities|Array|SetArrayElem (Variables|Default|GetHasUIDList) UID false))

(fn CopyHasUIDList
  (Utilities|Array|Clear (Variables|Default|GetHasUIDList_Main))
  (for _array_element (Variables|Default|GetHasUIDList)
    (Utilities|Array|Add (Variables|Default|GetHasUIDList_Main) _array_element)))

(fn GetUIDMain
  (bind _hasuidlist_main (Variables|Default|GetHasUIDList_Main))
  (for (_array_element _array_index) _hasuidlist_main
    (if (not _array_element)
      (Utilities|Array|SetArrayElem _hasuidlist_main _array_index true)
      (return _array_index))))