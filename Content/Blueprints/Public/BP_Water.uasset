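; BP_Water is a rising water hazard that flags the player character on contact.
; On BeginPlay it derives Speed from its start height, FullZ and Time, then registers itself with BP_MainGM.
; Tick moves it up by local offset while Rising is true, with no check against FullZ here.
; Box overlap sets WAterHit on BP_PlayerCharacter_DH and prints a respawn debug message.
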(event OnComponentBeginOverlap(Box)
  (params (OverlappedComponent :type Primitive%20Component%20Object%20Reference) (OtherActor :type Actor%20Object%20Reference) (OtherComp :type Primitive%20Component%20Object%20Reference) (OtherBodyIndex :type Integer) (bFromSweep :type Boolean) (SweepResult :type Hit%20Result%20Structure%20%28by%20ref%29))
  (bind _asbp_player_character_dh (Utilities|Casting|CastToBP_PlayerCharacter_DH OtherActor))
  (Variables|/Game/Blueprints/Hunter_DH/BP_PlayerCharacter_DH.BP_PlayerCharacter_DH_C|SetWAterHit _asbp_player_character_dh true)
  (Development|PrintString "리스폰"))

(event EventBeginPlay
  (Variables|Default|SetRising true)
  (Variables|Default|SetInitialZ (.z (Transformation|GetActorLocation)))
  (Variables|Default|Setspeed (/ (- (Variables|Default|GetFullZ) (Variables|Default|GetInitialZ)) (Variables|Default|GetTime)))
  (bind _asbp_main_gm (Utilities|Casting|CastToBP_MainGM (Game|GetGameMode)))
  (Variables|/Game/Blueprints/System/Main/BP_MainGM.BP_MainGM_C|Setwater _asbp_main_gm self))

(event EventTick
  (params (DeltaSeconds :type Float%20%28single-precision%29))
  (if (Variables|Default|GetRising)
    (Transformation|AddActorLocalOffset (Math|Vector|MakeVector 0.0 0.0 (* DeltaSeconds (Variables|Default|Getspeed))) false false)))

(fn ConstructionScript)