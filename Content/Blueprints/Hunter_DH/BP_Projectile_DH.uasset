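; Projectile actor in the Hunter_DH set that flies as a bullet without gravity and expires after its configured lifetime.
; On sphere overlap it calls ApplyDamage on the other actor, crediting player controller 0, and spawns a scaled-up hit emitter at the sphere's location.
; The overlap does not destroy the projectile, and the BulletMove event only reassigns the movement component to itself.
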(event OnComponentBeginOverlap(Sphere)
  (params (OverlappedComponent :type Primitive%20Component%20Object%20Reference) (OtherActor :type Actor%20Object%20Reference) (OtherComp :type Primitive%20Component%20Object%20Reference) (OtherBodyIndex :type Integer) (bFromSweep :type Boolean) (SweepResult :type Hit%20Result%20Structure%20%28by%20ref%29))
  (Game|Damage|ApplyDamage OtherActor 0.0 (Game|GetPlayerController 0) self)
  (Effects|SpawnEmitteratLocation "/Game/Resources/Hunter/FX/UseHit.UseHit" (Transformation|GetWorldLocation (Variables|Default|GetSphere)) "0, 0, 0" "5.000000,5.000000,5.000000"))

(event Custom|BulletMove
  ;[1 1 1] Bullet
  (bind _output_get (Variables|총알|SetProjectileMovement (Variables|총알|GetProjectileMovement))))

(event EventBeginPlay
  ;[1 1 1] Bullet
  (Variables|/Script/Engine.ProjectileMovementComponent|SetProjectileGravityScale (stale Custom|BulletMove _output_get) 0.0)
  (Actor|SetLifeSpan (Variables|Default|GetBulletLife)))

(fn ConstructionScript)