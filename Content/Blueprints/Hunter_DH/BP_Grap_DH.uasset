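; Grapple projectile that gives the player an anchor point when it hits something.
; Each tick it zeroes projectile gravity and moves its secondary Box1 component to the player's location.
; A Box hit sets GrapCheck and passes the projectile's location to MyPlayer as GrapPoint, then clears the flag and destroys itself after a delay.
; If nothing is hit shortly after spawning, it destroys itself.
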(event OnComponentHit(Box)
  (params (HitComponent :type Primitive%20Component%20Object%20Reference) (OtherActor :type Actor%20Object%20Reference) (OtherComp :type Primitive%20Component%20Object%20Reference) (NormalImpulse :type Vector :default "0, 0, 0") (Hit :type Hit%20Result%20Structure%20%28by%20ref%29))
  (bind _myplayer (Variables|Default|GetMyPlayer))
  ;[1 1 1] 그랩 투사체가 다른 지형에 붙착시 붙착화인
  (Development|PrintString "Grap")
  (Variables|Default|SetHitCK true)
  ;[1 1 1] 플레이어에게 그랩 성공 확인
  (Variables|/Game/Blueprints/Hunter_DH/BP_PlayerCharacter_DH.BP_PlayerCharacter_DH_C|SetGrapCheck _myplayer true)
  ;[1 1 1] 지금 그랩 포인트 위치를 플레이어에게 전달 딜레이후 삭제
  (Variables|/Game/Blueprints/Hunter_DH/BP_PlayerCharacter_DH.BP_PlayerCharacter_DH_C|SetGrapPoint _myplayer (Transformation|GetActorLocation))
  (Utilities|FlowControl|Delay 3.0)
  (Variables|/Game/Blueprints/Hunter_DH/BP_PlayerCharacter_DH.BP_PlayerCharacter_DH_C|SetGrapCheck _myplayer false)
  (Actor|DestroyActor))

(event Custom|BulletMove
  (bind _output_get (Variables|Default|SetProjectileMovement (Variables|Default|GetProjectileMovement))))

(event EventBeginPlay
  ;[1 1 1] 채공시간까지 타겟에 붙지 않으면 그랩 포인트 삭제
  (Utilities|FlowControl|Delay 0.5)
  (if (not (Variables|Default|GetHitCK))
    (Development|PrintString "GrapDelte")
    (Actor|DestroyActor)))

(event EventTick
  (params (DeltaSeconds :type Float%20%28single-precision%29))
  ;[1 1 1] 매틱마다플레이어 확인
  (bind _asbp_player_character_dh (Utilities|Casting|CastToBP_PlayerCharacter_DH (Game|GetPlayerCharacter 0)))
  ;[1 1 1] 고정 스피어 위치 플레이어 와 동일하게 변경
  (Transformation|SetWorldLocation (Variables|Default|GetBox1) (Transformation|GetActorLocation _asbp_player_character_dh) false false)
  (Variables|/Script/Engine.ProjectileMovementComponent|SetProjectileGravityScale (stale Custom|BulletMove _output_get) 0.0))

(fn ConstructionScript)