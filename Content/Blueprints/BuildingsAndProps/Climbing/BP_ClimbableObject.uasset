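; BP_ClimbableObject is a VR climbable prop that lets the player pull their pawn around by gripping it with motion controllers.
; Climbing and Letgo events track up to two gripping controllers, storing the newest or remaining hand's world position as the pivot.
; While selected, Tick offsets the pawn by the pivot-to-hand difference, without sweep, so the body moves opposite the hand.
; With two hands, the second drives movement and is snapped back to the pivot.
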(event EventTick
  (params (DeltaSeconds :type Float%20%28single-precision%29))
  (bind _secondmotioncontroller (Variables|Default|GetSecondMotionController))
  ;[1 1 1] tick
  (Utilities|FlowControl|Sequence
    (:then_0
      (|CallParentFunction 0.0))
    (:then_1
      (Utilities|IsValid (Variables|Default|GetVRPawn)
        (:Is%20Valid
          (if (Variables|Default|GetIsSelected)
            (Utilities|IsValid (Variables|Default|GetFirstMotionController)
              (:Is%20Valid
                (Utilities|IsValid (Variables|Default|GetSecondMotionController)
                  (:Is%20Valid
                    (Transformation|AddActorWorldOffset (Variables|Default|GetVRPawn) (- (Variables|Default|GetPivotPoint) (Transformation|GetWorldLocation _secondmotioncontroller)))
                    (Transformation|SetWorldLocation _secondmotioncontroller (Variables|Default|GetPivotPoint) false false))
                  (:Is%20Not%20Valid
                    (Transformation|AddActorWorldOffset (Variables|Default|GetVRPawn) (- (Variables|Default|GetPivotPoint) (Transformation|GetWorldLocation (Variables|Default|GetFirstMotionController))))))))))))))

(event EventClimbing
  (params (Motion%20Controller :type Scene%20Component%20Object%20Reference))
  ;[1 1 1] climbing
  (Utilities|IsValid Motion%20Controller
    (:Is%20Valid
      (Utilities|IsValid (Variables|Default|GetFirstMotionController)
        (:Is%20Valid
          (if (!= (Variables|Default|GetFirstMotionController) Motion%20Controller)
            (Variables|Default|SetSecondMotionController Motion%20Controller)
            (Variables|Default|SetPivotPoint (Transformation|GetWorldLocation (select (Utilities|IsValid (Variables|Default|GetSecondMotionController)) (Variables|Default|GetSecondMotionController) (Variables|Default|GetFirstMotionController))) :!label _label)
            (Variables|Default|SetVRPawn (Game|Player|GetPlayerPawn 0))))
        (:Is%20Not%20Valid
          (Variables|Default|SetFirstMotionController Motion%20Controller)
          (goto _label))))))

(event EventLetgo
  (params (Motion%20Controller :type Scene%20Component%20Object%20Reference))
  ;[1 1 1] letgo
  (Utilities|IsValid (Variables|Default|GetSecondMotionController)
    (:Is%20Valid
      (if (== Motion%20Controller (Variables|Default|GetSecondMotionController))
        (Variables|Default|SetSecondMotionController 0)
        (Variables|Default|SetPivotPoint (Transformation|GetWorldLocation (Variables|Default|GetFirstMotionController)))
        (else
          (Variables|Default|SetFirstMotionController (Variables|Default|GetSecondMotionController))
          (Variables|Default|SetSecondMotionController 0)
          (Variables|Default|SetPivotPoint (Transformation|GetWorldLocation (Variables|Default|GetFirstMotionController))))))
    (:Is%20Not%20Valid
      (if (== Motion%20Controller (Variables|Default|GetFirstMotionController))
        (Variables|Default|SetFirstMotionController 0)
        (Variables|Default|SetSecondMotionController 0)
        (Variables|Default|SetPivotPoint "0, 0, 0")
        (Variables|Default|SetVRPawn 0)))))

(fn ConstructionScript)