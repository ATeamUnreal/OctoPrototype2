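; Breakable prop that shatters when it takes damage whose causer is a BP_MotionControllerMain.
; Damage is handled only on the authority, with the Box collision state guarding against repeat breaks.
; Destruction disables the box, hides the static mesh and spawns a separate BP_Breakable_DM actor, passing it the destructible mesh, lifetime and original mesh transform.
; The original actor then destroys itself.
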(event Custom|Destruction
  (Collision|SetCollisionEnabled (Variables|Default|GetBox) "NoCollision")
  (Rendering|SetVisibility (Variables|Default|GetStaticMesh) false false)
  (bind _returnvalue (Game|SpawnActorfromClass "/Game/Blueprints/BuildingsAndProps/Breakable/BP_Breakable_DM.BP_Breakable_DM_C" (Transformation|GetActorTransform) "AlwaysSpawn" 0 0))
  (Default|Destruction _returnvalue (Variables|Default|GetDMLifeTime) (Variables|Default|GetDestructibleMesh) (Transformation|GetWorldTransform (Variables|Default|GetStaticMesh)))
  (Actor|DestroyActor))

(event Game|Damage|EventAnyDamage
  (params (Damage :type Float%20%28single-precision%29) (DamageType :type Damage%20Type%20Object%20Reference) (InstigatedBy :type Controller%20Object%20Reference) (DamageCauser :type Actor%20Object%20Reference))
  ;[1 1 1] 데미지를 받으면 부서짐
  (Networking|SwitchHasAuthority
    (:Authority
      (Utilities|Casting|CastToBP_MotionControllerMain DamageCauser)
      (if (not (Utilities|Enum|Equal(Enum) (Collision|GetCollisionEnabled (Variables|Default|GetBox)) "NoCollision"))
        (CallFunction|Destruction)))))

(fn ConstructionScript)