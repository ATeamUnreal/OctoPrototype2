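; BP_PickupObject is a physics prop that can be picked up and dropped.
; Pickup disables physics on its Box, attaches the root to the given component keeping world transform, and sets IsUsing.
; Drop re-enables physics, detaches the actor, clears IsUsing and sets IsDropped, whose RepNotify is empty.
; Tick calls Drop whenever the object is not in use and has a valid parent component.
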(event EventTick
  (params (DeltaSeconds :type Float%20%28single-precision%29))
  ;[1 1 1] Tick
  (|CallParentFunction DeltaSeconds)
  (if (not (Variables|Default|GetIsUsing))
    (Utilities|IsValid (Class|Actor|GetParentComponent)
      (:Is%20Valid
        (CallFunction|Drop "0, 0, 0")))))

(event EventPickup
  (params (AttachTo :type Scene%20Component%20Object%20Reference))
  ;[1 1 1] Pickup
  (Physics|SetSimulatePhysics (Variables|Default|GetBox) false)
  (Transformation|AttachComponentToComponent (Variables|Transformation|GetRootComponent) AttachTo "None" "KeepWorld" "KeepWorld" "KeepWorld" false)
  (Variables|Default|SetIsUsing true))

(event EventDrop
  (params (Velocity :type Vector :default "0, 0, 0"))
  ;[1 1 1] Pickup
  (Physics|SetSimulatePhysics (Variables|Default|GetBox) true)
  (Transformation|DetachFromActor "KeepWorld" "KeepWorld" "KeepWorld")
  (Variables|Interactable|SetIsDropped true)
  (Variables|Default|SetIsUsing false))

(fn ConstructionScript)

(fn OnRepIsDropped)