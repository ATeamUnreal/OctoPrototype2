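; Main game mode that assigns each joining player either the VR role or a PC player role.
; On PostLogin, the first player gets a BP_VRPawnMain at the "OctoStart" actor if a headset is enabled.
; All others get a PCPlayer at a "HunterStart" actor picked by the shared PlayerIndex counter, so HunterStart index 0 is skipped when the VR pawn spawns.
; Each spawned pawn is possessed immediately.
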(event EventPostLogin
  (params (NewPlayer :type Player%20Controller%20Object%20Reference))
  (if (and (Class|HeadMountedDisplayFunctionLibrary|IsHeadMountedDisplayEnabled) (< (Variables|Default|GetPlayerIndex) 1))
    (bind _outactors (Actor|GetAllActorswithTag "OctoStart"))
    (bind _returnvalue (Game|SpawnActorfromClass "/Game/Blueprints/Octopus/BP_VRPawnMain.BP_VRPawnMain_C" (Transformation|GetActorTransform (Utilities|Array|Get(acopy) _outactors)) "AlwaysSpawn" 0 0))
    (Variables|/Game/Blueprints/Octopus/BP_VRPawnMain.BP_VRPawnMain_C|SetIsDebugMode _returnvalue (not (Class|HeadMountedDisplayFunctionLibrary|IsHeadMountedDisplayEnabled)))
    (Pawn|Possess NewPlayer _returnvalue)
    (Math|Integer|IncrementInt (Variables|Default|GetPlayerIndex))
    (else
      (bind _outactors_2 (Actor|GetAllActorswithTag "HunterStart"))
      (bind _returnvalue_2 (Game|SpawnActorfromClass (Variables|Default|GetPCPlayer) (Transformation|GetActorTransform (Utilities|Array|Get(acopy) _outactors_2 (Variables|Default|GetPlayerIndex))) "AlwaysSpawn" 0 0))
      (Pawn|Possess NewPlayer _returnvalue_2)
      (Math|Integer|IncrementInt (Variables|Default|GetPlayerIndex)))))

(event EventBeginPlay)

(fn ConstructionScript)