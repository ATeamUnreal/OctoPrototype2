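; Physics-simulated pickup object that can be grabbed, carried and dropped, in the Octopus blueprints folder.
; Pickup turns off physics on the Box and attaches the root to a given component, keeping its world transform; Drop detaches it and re-enables physics.
; Highlight swaps the mesh's first material to a gripable material, and HighlightBack restores the original material cached on BeginPlay.
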(event EventBeginPlay
  (Variables|Default|SetOriginalMaterial (Utilities|Array|Get(acopy) (Rendering|Material|GetMaterials (Variables|Default|GetStaticMesh)))))

(event EventHighlight
  (Rendering|Material|SetMaterial (Variables|Default|GetStaticMesh) 0 (Variables|Default|GetGripableMaterial)))

(event EventHighlightBack
  (Rendering|Material|SetMaterial (Variables|Default|GetStaticMesh) 0 (Variables|Default|GetOriginalMaterial)))

(event EventPickup
  (params (AttachTo :type Scene%20Component%20Object%20Reference))
  (Physics|SetSimulatePhysics (Variables|Default|GetBox) false)
  (Transformation|AttachComponentToComponent (Variables|Transformation|GetRootComponent) AttachTo "None" "KeepWorld" "KeepWorld" "KeepWorld" false))

(event EventDrop
  (Physics|SetSimulatePhysics (Variables|Default|GetBox) true)
  (Transformation|DetachFromActor "KeepWorld" "KeepWorld" "KeepWorld"))

(fn ConstructionScript)