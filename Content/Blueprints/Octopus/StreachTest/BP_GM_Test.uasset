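; Test game mode in the Octopus StreachTest folder that handles player login and character respawning.
; PostLogin increments a player counter and, only when the counter equals 1, looks up actors by class and calls Possess on the new player.
; RespawnCharacter spawns a BP_PlayerCharacter_SN at a random actor tagged Respawn, ignoring collisions, without possessing it.
; A CreatePlayer call is left disconnected and never runs.
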(event Custom|RespawnCharacter
  (bind _outactors (Actor|GetAllActorswithTag "Respawn"))
  (Game|SpawnActorfromClass "/Game/SN/Blueprints_SN/BP_PlayerCharacter_SN.BP_PlayerCharacter_SN_C" (Transformation|GetActorTransform (Utilities|Array|Get(acopy) _outactors (Math|Random|RandomIntegerinRange 0 (- (Utilities|Array|Length _outactors) 1)))) "AlwaysSpawn" 0 0))

(event EventBeginPlay)

(event EventPostLogin
  (params (NewPlayer :type Player%20Controller%20Object%20Reference))
  ;[1 1 1] 코멘트
  (if (== (Variables|Default|GetPlayerNumber) 1)
    (bind _outactors (Actor|GetAllActorsOfClass 0))
    (Pawn|Possess NewPlayer)
    (Math|Integer|IncrementInt (Variables|Default|GetPlayerNumber))
    (else
      (Math|Integer|IncrementInt (Variables|Default|GetPlayerNumber)))))

(fn ConstructionScript)