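; Test throwable object that breaks when its Box component takes a hard enough hit.
; A hit impulse above a fixed threshold triggers Destruction, which disables box collision and hides the static mesh.
; It then spawns a separate BP_Breakable_DM actor at its transform, hands it the destructible mesh and lifetime to handle the breakage, and destroys itself.
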(event OnComponentHit(Box)
  (params (HitComponent :type Primitive%20Component%20Object%20Reference) (OtherActor :type Actor%20Object%20Reference) (OtherComp :type Primitive%20Component%20Object%20Reference) (NormalImpulse :type Vector :default "0, 0, 0") (Hit :type Hit%20Result%20Structure%20%28by%20ref%29))
  ;[1 1 1] 일정 이상의 충격이 가해지면 부서짐
  (if (> (Math|Vector|VectorLength NormalImpulse) 7e+05)
    (CallFunction|Destruction)))

(event Custom|Destruction
  ;[1 1 1] 부서짐 효과
  (Collision|SetCollisionEnabled (Variables|Default|GetBox) "NoCollision")
  (Rendering|SetVisibility (Variables|Default|GetStaticMesh) false false)
  (bind _returnvalue (Game|SpawnActorfromClass "/Game/Blueprints/Props/Breakable/BP_Breakable_DM.BP_Breakable_DM_C" (Transformation|GetActorTransform) "AlwaysSpawn" 0 0))
  (Default|Destruction _returnvalue (Variables|Default|GetDMLifeTime) (Variables|Default|GetDestructibleMesh))
  (Actor|DestroyActor))

(fn ConstructionScript
  (|CallParentFunction))