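; Test climbable VR object that lets the player pull their pawn around by gripping it and highlights when targeted.
; Climbing stores the gripping motion controller and a pivot point; Tick offsets the pawn by the controller's drift and snaps the controller back to the pivot.
; Letgo handles hand-over or clears the grip, though Climbing only ever clears the second controller slot, never fills it.
; Highlight events swap the mesh material.
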(event EventBeginPlay
  ;[1 1 1] init
  (Variables|Default|SetOriginalMaterial (Utilities|Array|Get(acopy) (Rendering|Material|GetMaterials (Variables|Default|GetStatic%20Mesh)))))

(event EventClimbing
  (params (Motion%20Controller :type Scene%20Component%20Object%20Reference))
  (if (Utilities|IsValid (Variables|Default|GetFirstMotionController))
    (Variables|Default|SetSecondMotionController 0)
    (else
      (Variables|Default|SetFirstMotionController Motion%20Controller)))
  (Variables|Default|SetPivotPoint (Transformation|GetWorldLocation (select (Utilities|IsValid (Variables|Default|GetSecondMotionController)) (Variables|Default|GetSecondMotionController) (Variables|Default|GetFirstMotionController))))
  (Variables|Default|SetVRPawn (Game|Player|GetPlayerPawn 0)))

(event EventLetgo
  (params (Motion%20Controller :type Scene%20Component%20Object%20Reference))
  (if (Utilities|IsValid (Variables|Default|GetSecondMotionController))
    (if (== Motion%20Controller (Variables|Default|GetSecondMotionController))
      (Variables|Default|SetSecondMotionController 0)
      (Variables|Default|SetPivotPoint (Transformation|GetWorldLocation (Variables|Default|GetFirstMotionController)))
      (else
        (Variables|Default|SetFirstMotionController (Variables|Default|GetSecondMotionController))
        (Variables|Default|SetSecondMotionController 0)
        (Variables|Default|SetPivotPoint (Transformation|GetWorldLocation (Variables|Default|GetFirstMotionController)))))
    (elif (== Motion%20Controller (Variables|Default|GetFirstMotionController))
      (Variables|Default|SetFirstMotionController 0)
      (Variables|Default|SetSecondMotionController 0)
      (Variables|Default|SetPivotPoint "0, 0, 0"))))

(event EventHighlight
  ;[1 1 1] interactable highlight
  (Rendering|Material|SetMaterial (Variables|Default|GetStatic%20Mesh) 0 (Variables|Default|GetGripableMaterial)))

(event EventHighlightBack
  ;[1 1 1] interactable highlight
  (Rendering|Material|SetMaterial (Variables|Default|GetStatic%20Mesh) 0 (Variables|Default|GetOriginalMaterial)))

(event EventTick
  (params (DeltaSeconds :type Float%20%28single-precision%29))
  (bind _firstmotioncontroller (Variables|Default|GetFirstMotionController))
  (bind _secondmotioncontroller (Variables|Default|GetSecondMotionController))
  (bind _secondmotioncontroller_2 (Variables|Default|GetSecondMotionController))
  (bind _returnvalue (Utilities|IsValid _secondmotioncontroller_2))
  (bind _returnvalue_2 (select _returnvalue _secondmotioncontroller _firstmotioncontroller))
  (Utilities|IsValid (Variables|Default|GetVRPawn)
    (:Is%20Valid
      (Utilities|IsValid (Variables|Default|GetFirstMotionController)
        (:Is%20Valid
          (bind _asbp_vrpawn_main (Utilities|Casting|CastToBP_VRPawnMain (Variables|Default|GetVRPawn))
            (:then
              (if (Variables|/Game/Blueprints/Octopus/BP_VRPawnMain.BP_VRPawnMain_C|GetIsClimbing _asbp_vrpawn_main)
                (if (Rendering|IsVisible (Variables|Default|GetFirstMotionController)) :!label _label
                  (Transformation|AddActorWorldOffset (Variables|Default|GetVRPawn) (- (Variables|Default|GetPivotPoint) (Transformation|GetWorldLocation _returnvalue_2)))
                  (Transformation|SetWorldLocation _returnvalue_2 (Variables|Default|GetPivotPoint) false false))))
            (:CastFailed
              (goto _label))))))))

(fn ConstructionScript)