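; BP_Breakable_Test is a test breakable actor that shatters into physics pieces when it takes any damage.
; On damage it hides the intact StaticMesh, then reveals the static mesh children of the Scene component, enabling physics simulation and physics-only collision on each.
; The actor destroys itself three seconds later.
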(event Game|Damage|EventAnyDamage
  (params (Damage :type Float%20%28single-precision%29) (DamageType :type Damage%20Type%20Object%20Reference) (InstigatedBy :type Controller%20Object%20Reference) (DamageCauser :type Actor%20Object%20Reference))
  (Rendering|SetVisibility (Variables|Default|GetStaticMesh) false false)
  (for _array_element (Components|GetChildrenComponents (Variables|Default|GetScene) false)
    (bind _asstatic_mesh_component (Utilities|Casting|CastToStaticMeshComponent _array_element))
    (Rendering|SetVisibility _asstatic_mesh_component true false)
    (Physics|SetSimulatePhysics _asstatic_mesh_component true)
    (Collision|SetCollisionEnabled _asstatic_mesh_component "PhysicsOnly"))
  (Utilities|FlowControl|Delay 3.0)
  (Actor|DestroyActor))

(fn ConstructionScript
  (|CallParentFunction))