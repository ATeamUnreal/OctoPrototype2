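; Test motion controller Blueprint for a hand that grabs, climbs and stretches out to distant surfaces.
; Each tick it updates a grip state, shown as debug text, and picks and highlights an overlapping Interactable_Interface actor while open or able to grab.
; Grab and Release send pickup, climb, drop and let-go interface messages.
; Stretch line-traces, then detaches and teleports the hand sphere to the hit; stretching back reattaches it, with grabbing blocked briefly during each move.
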(event OnComponentBeginOverlap(Sphere)
  (params (OverlappedComponent :type Primitive%20Component%20Object%20Reference) (OtherActor :type Actor%20Object%20Reference) (OtherComp :type Primitive%20Component%20Object%20Reference) (OtherBodyIndex :type Integer) (bFromSweep :type Boolean) (SweepResult :type Hit%20Result%20Structure%20%28by%20ref%29))
  ;[1 1 1] 잡을 수 있는 오브젝트 하이라이트
)

(event OnComponentEndOverlap(Sphere)
  (params (OverlappedComponent :type Primitive%20Component%20Object%20Reference) (OtherActor :type Actor%20Object%20Reference) (OtherComp :type Primitive%20Component%20Object%20Reference) (OtherBodyIndex :type Integer))
  ;[1 1 1] 잡을수 있는 오브젝트 벗어나면 원복
)

(event Custom|Grab
  ;[1 1 1] Grab
  (Variables|Default|SetbWantsToGrip true)
  (Utilities|IsValid (Variables|Default|GetGripActor)
    (:Is%20Valid
      (Class|PickupActorInterface|Pickup(Message) (Variables|Default|GetGripActor) (Variables|Default|GetSphere))
      (Class|BPClimbinginterface|Climbing(Message) (Variables|Default|GetGripActor) (Variables|Default|GetMotionController))
      (Class|InteractableInterface|HighlightBack(Message) (Variables|Default|GetGripActor)))))

(event Custom|Release
  ;[1 1 1] Release
  (Variables|Default|SetbWantsToGrip false)
  (Utilities|IsValid (Variables|Default|GetGripActor)
    (:Is%20Valid
      (Class|PickupActorInterface|Drop(Message) (Variables|Default|GetGripActor))
      (Class|BPClimbinginterface|Letgo(Message) (Variables|Default|GetGripActor) (Variables|Default|GetMotionController))
      (Variables|Default|SetGripActor 0))))

(event Custom|Stretch
  (bind _staticmesh (Variables|Default|GetStaticMesh))
  ;[1 1 1] 팔 뻗기
  (if (Variables|Default|GetbIsStretched)
    (CallFunction|StretchBack)
    (else
      (switch Utilities|FlowControl|Switch|SwitchonGripEnum (Variables|Default|GetGripState)
        (:NewEnumerator0
          _)
        (:NewEnumerator1
          _))
      (bind (_outhit _returnvalue) (Collision|LineTraceForObjects (Transformation|GetWorldLocation _staticmesh) (* (Math|Vector|GetForwardVector _staticmesh) 1e+04) (Utilities|Array|MakeArray "ObjectTypeQuery1" "ObjectTypeQuery2") false 0 "None"))
      (if _returnvalue
        (Variables|Default|SetbIsStretching true)
        (Transformation|DetachFromComponent (Variables|Default|GetSphere) "KeepWorld" "KeepWorld" "KeepWorld" false)
        (Variables|Default|SetStretchTargetActor (.HitActor (Collision|BreakHitResult _outhit)))
        (Transformation|SetWorldLocation (Variables|Default|GetSphere) (.Location (Collision|BreakHitResult _outhit)) false false)
        (Utilities|FlowControl|Delay 0.5)
        (Variables|Default|SetbIsStretched true)
        (Variables|Default|SetbIsStretching false)))))

(event Custom|Stretch_Back
  ;[1 1 1] 팔 되돌리기
  (switch Utilities|FlowControl|Switch|SwitchonGripEnum (Variables|Default|GetGripState)
    (:NewEnumerator0
      _)
    (:NewEnumerator1
      _)
    (:NewEnumerator2
      _))
  (Variables|Default|SetbIsStretching true)
  (Transformation|AttachComponentToComponent (Variables|Default|GetSphere) (Variables|Default|GetStaticMesh) "None" "SnapToTarget" "SnapToTarget" "KeepWorld" true)
  (Transformation|SetRelativeLocation (Variables|Default|GetSphere) "60.000000, 0, 0" false false)
  (Utilities|FlowControl|Delay 0.5)
  (Variables|Default|SetbIsStretched false)
  (Variables|Default|SetbIsStretching false))

(event EventTick
  (params (DeltaSeconds :type Float%20%28single-precision%29))
  (Utilities|FlowControl|Sequence
    (:then_0
      ;[1 1 1] update - for debug
      (Rendering|Components|TextRender|SetText (Variables|Default|GetTextRender) (Utilities|Text|ToText(String) (Utilities|String|Append (Utilities|String|EnumtoString (Variables|Default|GetGripState)) " " (Utilities|GetDisplayName (Variables|Default|GetGripActor))))))
    (:then_1
      (CallFunction|GripStateUpdate))
    (:then_2
      (switch Utilities|FlowControl|Switch|SwitchonGripEnum (Variables|Default|GetGripState)
        (:NewEnumerator0
          _)
        (:NewEnumerator1
          _))
      (CallFunction|GetActorNearHand))
    (:then_3
      ;[1 1 1] 팔 스트레칭 업데이트
      (if (Variables|Default|GetbIsStretching)
        _))))

(fn ConstructionScript)

(fn GripStateUpdate
  (if (Variables|Default|GetbIsStretching)
    (Variables|Default|SetGripState "NewEnumerator3")
    (else
      (Utilities|IsValid (Variables|Default|GetGripActor)
        (:Is%20Valid
          (if (Variables|Default|GetbWantsToGrip)
            (Variables|Default|SetGripState "NewEnumerator2")
            (else
              (Variables|Default|SetGripState "NewEnumerator1"))))
        (:Is%20Not%20Valid
          (Variables|Default|SetGripState "NewEnumerator0"))))))

(fn GetActorNearHand
  (for _array_element (Collision|GetOverlappingActors (Variables|Default|GetSphere) "/Script/Engine.Actor" :!class /Script/Engine.PrimitiveComponent)
    (if (Utilities|DoesObjectImplementInterface _array_element "/Game/Blueprints/Octopus/StreachTest/Interactable_Interface.Interactable_Interface_C")
      (if (< (Math|Vector|Distance(Vector) (Transformation|GetWorldLocation (Variables|Default|GetSphere)) (Transformation|GetActorLocation _array_element)) (LocalVariables|GetNearestDist))
        (LocalVariables|SetNearestDist 0.0)
        (LocalVariables|SetNearestActor _array_element))))
  (Utilities|IsValid (LocalVariables|GetNearestActor)
    (:Is%20Valid
      (Utilities|IsValid (Variables|Default|GetGripActor)
        (:Is%20Valid
          (Class|InteractableInterface|HighlightBack(Message) (Variables|Default|GetGripActor)))
        (:Is%20Not%20Valid
          _))
      (Variables|Default|SetGripActor (LocalVariables|GetNearestActor))
      (Class|InteractableInterface|Highlight(Message) (LocalVariables|GetNearestActor))
      (return))))