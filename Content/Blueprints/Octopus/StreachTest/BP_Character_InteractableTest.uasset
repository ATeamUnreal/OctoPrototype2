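; Test character that VR motion controllers can highlight, pick up and throw, with HP shown on a text render.
; A PickupState machine (Normal, Selected, Hold, Dropped) drives it, with server-side Tick checks of overlapping controllers' GripActor swapping the highlight material.
; Authority-checked pickup and drop events call multicasts that toggle attachment, physics and movement, and a capsule hit after dropping restores walking.
; Damage lowers HP except while held; respawn test code is unconnected.
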(event OnComponentHit(CapsuleComponent)
  (params (HitComponent :type Primitive%20Component%20Object%20Reference) (OtherActor :type Actor%20Object%20Reference) (OtherComp :type Primitive%20Component%20Object%20Reference) (NormalImpulse :type Vector :default "0, 0, 0") (Hit :type Hit%20Result%20Structure%20%28by%20ref%29))
  ;[1 1 1] 던져지고 나서 땅에 떨어졌을 때
  ;;[1 1 1] Event
  (if (Utilities|Enum|Equal(Enum) (Variables|Interactable|GetPickupState) "NewEnumerator3")
    (CallFunction|DroppedServer)))

(event Custom|Dropped
  ;[1 1 1] 던져지고 나서 땅에 떨어졌을 때
  ;;[1 1 1] 멀티캐스트
  (Physics|SetSimulatePhysics (Variables|Default|GetCapsuleComponent) false)
  (Transformation|SetActorRotation (Math|Rotator|MakeRotator 0.0 (.pitch (Transformation|GetActorRotation)) 0.0))
  (Pawn|Components|CharacterMovement|SetMovementMode (Variables|Character|GetCharacterMovement) "MOVE_Walking" 0))

(event Custom|DroppedServer
  ;[1 1 1] 던져지고 나서 땅에 떨어졌을 때
  ;;[1 1 1] 서버에서 실행
  (Networking|SwitchHasAuthority
    (:Authority
      (Variables|Interactable|SetPickupState "NewEnumerator0")
      (CallFunction|Dropped))))

(event Custom|UpdateHPbar
  ;[1 1 1] hp
  (Rendering|Components|TextRender|SetText (Variables|Default|GetTextRender) (Utilities|Text|ToText(Float) (Variables|Default|Gethp) "HalfToEven")))

(event Custom|highlightUpdate
  ;[1 1 1] 컨트롤러가 잡으려고 할 때 하이라이트 / 아니면 원래대로
  (Networking|SwitchHasAuthority
    (:Authority
      (Utilities|FlowControl|Sequence
        (:then_0
          (switch Utilities|FlowControl|Switch|SwitchonEPickupObjState (Variables|Interactable|GetPickupState)
            (:NewEnumerator0
              _)
            (:NewEnumerator1
              _))
          (bind _isselected (CallFunction|FindIsSelected))
          (if _isselected
            (Variables|Interactable|SetPickupState "NewEnumerator1")
            (else
              (Variables|Interactable|SetPickupState "NewEnumerator0"))))
        (:then_1
          (switch Utilities|FlowControl|Switch|SwitchonEPickupObjState (Variables|Interactable|GetPickupState)
            (:NewEnumerator0
              (CallFunction|HighlightBack :!label _label))
            (:NewEnumerator1
              (CallFunction|Highlight :!label _label_2))
            (:NewEnumerator2
              (goto _label_2))
            (:NewEnumerator3
              (goto _label))))
        (:then_2
          (CallFunction|DebugText))))))

(event Custom|DropMulticast
  (bind _capsulecomponent (Variables|Default|GetCapsuleComponent))
  ;[1 1 1] Drop
  ;;[1 1 1] Multicast
  (Collision|SetCollisionEnabled _capsulecomponent "QueryAndPhysics")
  (Physics|SetSimulatePhysics _capsulecomponent true)
  (Transformation|DetachFromActor "KeepWorld" "KeepWorld" "KeepWorld"))

(event Custom|DropServer
  ;[1 1 1] Drop
  ;;[1 1 1] Server
  (Networking|SwitchHasAuthority
    (:Authority
      (if (Utilities|Enum|Equal(Enum) (Variables|Interactable|GetPickupState) "NewEnumerator2")
        (Utilities|IsValid (Variables|Interactable|GetAttachedHand)
          (:Is%20Valid
            (Variables|Interactable|SetAttachedHand 0)
            (Variables|Interactable|SetPickupState "NewEnumerator3")
            (CallFunction|DropMulticast)))))))

(event Custom|PickupServer
  (params (NewParam :type Scene%20Component%20Object%20Reference))
  ;[1 1 1] Pickup
  ;;[1 1 1] Server
  (Networking|SwitchHasAuthority
    (:Authority
      (if (Utilities|Enum|Equal(Enum) (Variables|Interactable|GetPickupState) "NewEnumerator1")
        (Variables|Interactable|SetAttachedHand NewParam)
        (Variables|Interactable|SetPickupState "NewEnumerator2")
        (CallFunction|PickupMulticast)))))

(event Custom|PickupMulticast
  ;[1 1 1] Pickup
  ;;[1 1 1] multicast
  (Physics|SetSimulatePhysics (Variables|Default|GetCapsuleComponent) false)
  (Transformation|AttachComponentToComponent (Variables|Transformation|GetRootComponent) (Variables|Interactable|GetAttachedHand) "None" "KeepWorld" "KeepWorld" "KeepWorld" false)
  (Pawn|Components|CharacterMovement|SetMovementMode (Variables|Character|GetCharacterMovement) "MOVE_None" 0))

(event Custom|debugText
  ;[1 0 0.913] for debug
  (Rendering|Components|TextRender|SetText (Variables|Default|GetTextRender1) (Utilities|Text|ToText(String) (Utilities|String|EnumtoString (Variables|Interactable|GetPickupState)))))

(event EventBeginPlay
  ;[1 1 1] BeginPlay - 원래 머터리얼 가져오기
  (|CallParentFunction)
  (Networking|SwitchHasAuthority
    (:Authority
      (Variables|Interactable|SetOriginalMaterial (Utilities|Array|Get(acopy) (Rendering|Material|GetMaterials (Variables|Character|GetMesh))))
      (CallFunction|UpdateHPbar))))

(event EventHighlight
  ;[1 1 1] highlight
  (Rendering|Material|SetMaterial (Variables|Character|GetMesh) 0 (Variables|Interactable|GetSelectedMatarial)))

(event EventPickup
  (params (AttachTo :type Scene%20Component%20Object%20Reference))
  ;[1 1 1] Pickup
  ;;[1 1 1] Event
  (CallFunction|PickupServer AttachTo))

(event EventDrop
  (params (Velocity :type Vector :default "0, 0, 0"))
  ;[1 1 1] Drop
  ;;[1 1 1] Event
  (CallFunction|DropServer))

(event EventHighlightBack
  ;[1 1 1] highlight
  (Rendering|Material|SetMaterial (Variables|Character|GetMesh) 0 (Variables|Interactable|GetOriginalMaterial)))

(event EventTick
  (params (DeltaSeconds :type Float%20%28single-precision%29))
  ;[1 1 1] Tick
  (|CallParentFunction DeltaSeconds)
  (CallFunction|HighlightUpdate))

(event Game|Damage|EventAnyDamage
  (params (Damage :type Float%20%28single-precision%29) (DamageType :type Damage%20Type%20Object%20Reference) (InstigatedBy :type Controller%20Object%20Reference) (DamageCauser :type Actor%20Object%20Reference))
  ;[1 1 1] Damage
  (|CallParentFunction Damage DamageType InstigatedBy DamageCauser)
  (switch Utilities|FlowControl|Switch|SwitchonEPickupObjState (Variables|Interactable|GetPickupState)
    (:NewEnumerator0
      _)
    (:NewEnumerator1
      _)
    (:NewEnumerator3
      _))
  (Variables|Default|Sethp (- (Variables|Default|Gethp) Damage))
  (CallFunction|UpdateHPbar))

(fn ConstructionScript)

(fn OnRepHp)

(fn OnRepIsDropped)

(fn OnRepIsSelected)

(fn OnRepAttachedHand)

(fn FindIsSelected
  (bind _capsulecomponent (Variables|Default|GetCapsuleComponent))
  (bind _overlappingactors (Collision|GetOverlappingActors _capsulecomponent "/Game/Blueprints/Octopus/BP_MotionControllerMain.BP_MotionControllerMain_C" :!class /Script/Engine.PrimitiveComponent))
  (LocalVariables|SetSelected false)
  (if (> (Utilities|Array|Length _overlappingactors) 0)
    (for _array_element _overlappingactors
      (bind _asbp_motion_controller_main (Utilities|Casting|CastToBP_MotionControllerMain _array_element))
      (if (== (Variables|/Game/Blueprints/Octopus/BP_MotionControllerMain.BP_MotionControllerMain_C|GetGripActor _asbp_motion_controller_main) self)
        (LocalVariables|SetSelected true)))
    (if (LocalVariables|GetSelected)
      (return true)
      (else
        (return false)))
    (else
      (return false))))

(fn OnRepPickupState)