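; Lobby game mode that spawns and possesses a pawn for each player on PostLogin.
; The first player gets the VR pawn if an HMD is enabled; otherwise players get the GameInstance's default hunter class.
; GetStartPoint checks the local HMD state for every login, returning the first OctoStart actor if enabled, else taking cached HunterStart actors in reverse order by player index.
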(event EventPostLogin
  (params (NewPlayer :type Player%20Controller%20Object%20Reference))
  (bind _asbp_gi (Utilities|Casting|CastToBP_GI (Game|GetGameInstance)))
  (bind _start (CallFunction|GetStartPoint))
  (bind _returnvalue (Game|SpawnActorfromClass (Utilities|Select :Index (Variables|Default|GetPlayerIndex) :Option%200 (select (Class|HeadMountedDisplayFunctionLibrary|IsHeadMountedDisplayEnabled) "/Game/Blueprints/Octopus/BP_VRPawnMain.BP_VRPawnMain_C" (Variables|/Game/Blueprints/Public/BP_GI.BP_GI_C|GetDefaultHunterClass _asbp_gi)) :Option%201 (Variables|/Game/Blueprints/Public/BP_GI.BP_GI_C|GetDefaultHunterClass _asbp_gi) :Option%202 (Variables|/Game/Blueprints/Public/BP_GI.BP_GI_C|GetDefaultHunterClass _asbp_gi) :Option%203 (Variables|/Game/Blueprints/Public/BP_GI.BP_GI_C|GetDefaultHunterClass _asbp_gi) :Option%204 (Variables|/Game/Blueprints/Public/BP_GI.BP_GI_C|GetDefaultHunterClass _asbp_gi)) (Transformation|GetActorTransform _start) "AlwaysSpawn" 0 0))
  (bind _aspawn (Utilities|Casting|CastToPawn _returnvalue))
  (Pawn|Possess NewPlayer _aspawn)
  (Math|Integer|IncrementInt (Variables|Default|GetPlayerIndex)))

(fn ConstructionScript)

(fn GetStartPoint
  (if (Class|HeadMountedDisplayFunctionLibrary|IsHeadMountedDisplayEnabled)
    ;[1 1 1] VR시작위치
    (bind _outactors (Actor|GetAllActorswithTag "OctoStart"))
    (return (Utilities|Array|Get(acopy) _outactors))
    (else
      ;[1 1 1] 헌터 시작위치
      (if (== (Utilities|Array|Length (Variables|Default|GetHunterSpawnPoints)) 0)
        (bind _outactors_2 (Actor|GetAllActorswithTag "HunterStart"))
        (Variables|Default|SetHunterSpawnPoints _outactors_2))
      (return (Utilities|Array|Get(acopy) (Variables|Default|GetHunterSpawnPoints) (- (- (Utilities|Array|Length (Variables|Default|GetHunterSpawnPoints)) 1) (Variables|Default|GetPlayerIndex)))))))