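; Entry-level player controller that routes the player to the VR or third-person start level based on whether an HMD is enabled.
; On BeginPlay it sets the game instance's role state; non-VR players also get an entry or network-error widget according to EntryState.
; VR and normal-start paths wait briefly, then GotoStart opens the matching level.
; The network-error path shows the cursor and stays put.
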(event Custom|GotoStart
  (Default|SetEntryState (Variables|Default|GetGameInstance) "NewEnumerator0")
  (if (Class|HeadMountedDisplayFunctionLibrary|IsHeadMountedDisplayEnabled)
    (Game|OpenLevel(byName) "VRStart")
    (else
      (Game|OpenLevel(byName) "TPSStart"))))

(event EventBeginPlay
  (bind _asbp_gi (Utilities|Casting|CastToBP_GI (Game|GetGameInstance)))
  (Utilities|IsValid _asbp_gi
    (:Is%20Valid
      (bind _output_get (Variables|Default|SetGameInstance _asbp_gi))
      (if (Class|HeadMountedDisplayFunctionLibrary|IsHeadMountedDisplayEnabled)
        (Default|SetRoleState _asbp_gi "NewEnumerator0")
        (Utilities|FlowControl|Delay 5.0 :!label _label)
        (CallFunction|GotoStart)
        (else
          (Default|SetRoleState _asbp_gi "NewEnumerator1")
          (switch Utilities|FlowControl|Switch|SwitchonEntryState (Variables|/Game/Blueprints/Public/BP_GI.BP_GI_C|GetEntryState _output_get)
            (:NewEnumerator0
              (bind _returnvalue (UserInterface|CreateWidget "/Game/Blueprints/System/Entry/EntryWidget.EntryWidget_C"))
              (UserInterface|Viewport|AddtoViewport _returnvalue 0)
              (goto _label))
            (:NewEnumerator1
              (bind _returnvalue_2 (UserInterface|CreateWidget "/Game/Blueprints/System/Entry/NetworkErrorWidget.NetworkErrorWidget_C"))
              (UserInterface|Viewport|AddtoViewport _returnvalue_2 0)
              (Variables|Default|SetbShowMouseCursor true))))))))

(event EventTick
  (params (DeltaSeconds :type Float%20%28single-precision%29)))

(fn ConstructionScript)