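; Player controller for the main map of a VR-versus-hunters game, handling startup, result screens and map travel.
; BeginPlay streams in Game_SubLevel, then either sets the VR pawn's game mode or, without an HMD, moves the hunter to a GameMode spawn and builds widgets.
; Authority shows results on the VR pawn and loops over all controllers so owning clients show hunter result or loading UI.
; Lobby and restart show loading before servertravel.
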(event Custom|ShowResultHunters
  (params (IsHunterVictory :type Boolean))
  (bind _hunterresultwidget (Variables|Default|GetHunterResultWidget))
  ;[1 1 1] 헌터 결과 UI표시
  ; 서버의 헌터UI를 표시하는 것이 아니므로 소유 클라이언트에서 실행
  (Utilities|IsValid _hunterresultwidget
    (:Is%20Valid
      (Widget|SetVisibility _hunterresultwidget "Visible")
      (Default|ShowResult _hunterresultwidget IsHunterVictory))))

(event Custom|ShowLoading
  (bind _loadingwidget (Variables|Default|GetLoadingWidget))
  ;[1 1 1] 헌터 로딩 UI 표시
  ; 서버의 헌터UI를 표시하는 것이 아니므로 소유 클라이언트에서 실행
  (Utilities|IsValid _loadingwidget
    (:Is%20Valid
      (Widget|SetVisibility _loadingwidget "Visible"))))

(event Custom|GoToLobby
  ;[1 1 1] 맵 로딩 함수들
  (CallFunction|ShowLoadingtoClients)
  (Utilities|FlowControl|Delay 1.0)
  (Development|ExecuteConsoleCommand "servertravel/Game/Maps/Lobby" 0))

(event Custom|RestartGame
  ;[1 1 1] 맵 로딩 함수들
  (CallFunction|ShowLoadingtoClients)
  (Utilities|FlowControl|Delay 1.0)
  (Development|ExecuteConsoleCommand "servertravel/Game/Maps/Main" 0))

(event Custom|ShowResult
  (params (IsHunterVictory :type Boolean))
  (CallFunction|ShowResultServer IsHunterVictory)
  (CallFunction|ShowResulttoClients IsHunterVictory))

(event Custom|ShowLoadingToClients
  ;[1 1 1] 헌터 로딩 UI 표시 지시
  ; 서버가 가지고 있는 헌터들의 플레이어 콘트롤러에 foreach로 각각 uI를 표시하라고 지시한다
  (Networking|SwitchHasAuthority
    (:Authority
      (bind _outactors (Actor|GetAllActorsOfClass "BP_MainPC_C"))
      (for _array_element _outactors
        (CallFunction|ShowLoading _array_element)))))

(event Custom|ShowResultToClients
  (params (IsHunterVictory :type Boolean))
  ;[1 1 1] 헌터 결과 UI 표시 지시
  ; 서버가 가지고 있는 헌터들의 플레이어 콘트롤러에 foreach로 각각 uI를 표시하라고 지시한다
  (Networking|SwitchHasAuthority
    (:Authority
      (bind _outactors (Actor|GetAllActorsOfClass "BP_MainPC_C"))
      (for _array_element _outactors
        (CallFunction|ShowResultHunters _array_element IsHunterVictory)))))

(event Custom|ShowResultServer
  (params (IsHunterVictory :type Boolean))
  ;[1 1 1] VR 쪽 결과화면 표시
  (Networking|SwitchHasAuthority
    (:Authority
      (bind _asbp_vrpawn_main (Utilities|Casting|CastToBP_VRPawnMain (Game|Player|GetPlayerPawn 0)))
      (Utilities|IsValid _asbp_vrpawn_main
        (:Is%20Valid
          (Default|SetResultUI _asbp_vrpawn_main "Visible")
          (Default|ShowResult (Variables|/Game/Blueprints/Octopus/BP_VRPawnMain.BP_VRPawnMain_C|GetOctoResultWidget _asbp_vrpawn_main) IsHunterVictory))))))

(event EventBeginPlay
  (if (Class|HeadMountedDisplayFunctionLibrary|IsHeadMountedDisplayEnabled)
    (bind _asbp_vrpawn_main (Utilities|Casting|CastToBP_VRPawnMain (Game|Player|GetPlayerPawn 0)))
    (Game|LoadStreamLevel(byName) "Game_SubLevel" true)
    (Utilities|FlowControl|Delay 2.0)
    (Default|SetGameMode _asbp_vrpawn_main)
    (else
      ;[1 1 1] 로딩위젯 생성
      (bind _returnvalue (UserInterface|CreateWidget "/Game/Blueprints/System/Public/LoadingWidget.LoadingWidget_C"))
      (UserInterface|Viewport|AddtoViewport _returnvalue 0)
      (Variables|Default|SetLoadingWidget _returnvalue)
      (Input|SetIgnoreMoveInput false)
      (Game|LoadStreamLevel(byName) "Game_SubLevel" true)
      (Utilities|FlowControl|Delay 2.0)
      (bind _asbp_main_gm (Utilities|Casting|CastToBP_MainGM (Game|GetGameMode)))
      (bind _respawntransform (Default|GetHunterSpawnPoints _asbp_main_gm))
      (Transformation|SetActorTransform (Game|Player|GetPlayerPawn 0) _respawntransform)
      (Widget|SetVisibility (Variables|Default|GetLoadingWidget) "Collapsed")
      ;[1 1 1] 메인위젯 생성
      (bind _returnvalue_2 (UserInterface|CreateWidget "/Game/Blueprints/System/Main/MainWidget.MainWidget_C"))
      (UserInterface|Viewport|AddtoViewport _returnvalue_2 0)
      ;[1 1 1] 헌터 결과 화면 위젯 추가 생성시 숨김
      (bind _returnvalue_3 (UserInterface|CreateWidget "/Game/Blueprints/System/Main/HunterResultWidget.HunterResultWidget_C"))
      (UserInterface|Viewport|AddtoViewport _returnvalue_3 0)
      (bind _output_get (Variables|Default|SetHunterResultWidget _returnvalue_3))
      (Widget|SetVisibility _output_get "Collapsed")
      (Variables|Default|SetbShowMouseCursor false)
      (Input|SetInputModeGameOnly self))))

(event Input|KeyboardEvents|MotionControllerRightThumbstickLeft
  (params (Key :type Key%20Structure))
  (:Pressed
    (CallFunction|ShowResult false)))

(fn ConstructionScript)