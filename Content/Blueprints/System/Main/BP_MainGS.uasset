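; Main game state that tracks the hunters' respawn pool, a rising water level and reactions to game state changes.
; Respawn decrements and the count's OnRep refresh the first player controller's hunter widget, and running out calls GameOver on the game mode.
; Once initialized, water height climbs linearly on the authority's Tick until it passes its final height.
; Switching to Playing ends that controller's loading; a debug function prints every player's HP.
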(event Custom|DecreaseRespawnCount
  ;[1 1 1] 리스폰카운트 업데이트
  (Math|Integer|DecrementInt (Variables|Default|GetRespawnCount)
    (:%20%20
      ;;[1 1 1] 서버쪽에서의  UI업데이트
      (bind _asbp_main_pc (Utilities|Casting|CastToBP_MainPC (Game|GetPlayerController 0)))
      (Utilities|IsValid _asbp_main_pc
        (:Is%20Valid
          (Default|UpdateHunterMainWidgetServer _asbp_main_pc)
          (if (not (> (Variables|Default|GetRespawnCount) 0))
            (Variables|Default|SetRespawnCount 0)
            (bind _asbp_main_gm (Utilities|Casting|CastToBP_MainGM (Game|GetGameMode)))
            (Utilities|IsValid _asbp_main_gm
              (:Is%20Valid
                (Default|GameOver _asbp_main_gm false)))))))))

(event EventBeginPlay
  (CallFunction|InitRespawnCount))

(event EventTick
  (params (DeltaSeconds :type Float%20%28single-precision%29))
  ;[1 1 1] Tick
  (Networking|SwitchHasAuthority
    (:Authority
      (if (Variables|Water|GetWaterRising)
        (Variables|Water|SetWaterHeight (+ (Variables|Water|GetWaterHeight) (* DeltaSeconds (Variables|Water|GetWaterSpeed))))
        (if (> (Variables|Water|GetWaterHeight) (Variables|Water|GetWaterFinalZ))
          (Variables|Water|SetWaterRising false))))))

(event EventDowhenCurrentGameStateChanged
  (if (Utilities|Enum|Equal(Enum) (Variables|Default|GetCurrentGameState) "Playing")
    (Development|PrintString "set playing" true true "(R=0.000000,G=0.660000,B=1.000000,A=1.000000)" 2e+01)
    (bind _asbp_main_pc (Utilities|Casting|CastToBP_MainPC (Game|GetPlayerController 0)))
    (Default|EndLoadingServer _asbp_main_pc)))

(fn ConstructionScript)

(fn InitRespawnCount
  (Variables|Default|SetRespawnCount (Variables|Default|GetMaxRespawnCount)))

(fn InitWaterValues
  (params (InitialZ :type Float%20%28single-precision%29) (FullZ :type Float%20%28single-precision%29))
  (Variables|Water|SetWaterHeight InitialZ)
  (Variables|Water|SetWaterFinalZ FullZ)
  (Variables|Water|SetWaterSpeed (/ (- (Variables|Water|GetWaterFinalZ) (Variables|Water|GetWaterHeight)) (Variables|Water|GetWaterTime)))
  (Variables|Water|SetWaterRising true))

(fn Test
  (for _array_element (Variables|Default|GetPlayerArray)
    (bind _asbp_main_ps (Utilities|Casting|CastToBP_MainPS _array_element))
    (LocalVariables|SetdebugText (Utilities|String|Append (LocalVariables|GetdebugText) " " (Utilities|String|ToString(Float) (Variables|/Game/Blueprints/System/Main/BP_MainPS.BP_MainPS_C|GetCurrentHP _asbp_main_ps)))))
  (Development|PrintString (LocalVariables|GetdebugText)))

(fn OnRepRespawnCount
  (bind _asbp_main_pc (Utilities|Casting|CastToBP_MainPC (Game|GetPlayerController 0)))
  (Utilities|IsValid _asbp_main_pc
    (:Is%20Valid
      (Default|UpdateHunterMainWidgetServer _asbp_main_pc))))