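; Main game mode for an asymmetric match between a VR Octo player and Hunters, handling pawn spawning, Hunter respawns and game over.
; On login, the player state's role picks a VR pawn or the game instance's default Hunter class, placed by game state and role.
; Hunter spawns take a shuffled available respawn area, falling back to a random FinalSpawnPoint.
; GameOver fires only while Playing and shows the result on player controller 0.
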(event Custom|RespawnPawn
  (params (Hunter :type Pawn%20Object%20Reference))
  ;[1 1 1] 초기 폰 배치
  (bind _respawntransform (CallFunction|GetHunterSpawnPoints))
  (Transformation|SetActorTransform Hunter _respawntransform))

(event Custom|GameOver
  (params (IsHunterVictory :type Boolean))
  ;[1 1 1] 게임오버 처리
  (bind _asbp_main_gs (Utilities|Casting|CastToBP_MainGS (Game|GetGameState)))
  (if (Utilities|Enum|Equal(Enum) (Variables|/Game/Blueprints/System/Main/BP_MainGS.BP_MainGS_C|GetCurrentGameState _asbp_main_gs) "NewEnumerator1")
    (Variables|/Game/Blueprints/System/Main/BP_MainGS.BP_MainGS_C|SetCurrentGameState _asbp_main_gs "NewEnumerator2")
    (if IsHunterVictory
      (CallFunction|HunterWin)
      (else
        (CallFunction|OctoWin)))))

(event Custom|OctoWin
  ;[1 1 1] 게임오버 처리
  ;;[1 1 1] 게임오버시 결과 화면 처리
  (bind _asbp_main_pc (Utilities|Casting|CastToBP_MainPC (Game|GetPlayerController 0)))
  (Default|ShowResult _asbp_main_pc false))

(event Custom|HunterWin
  ;[1 1 1] 게임오버 처리
  ;;[1 1 1] 게임오버시 결과 화면 처리
  (bind _asbp_main_pc (Utilities|Casting|CastToBP_MainPC (Game|GetPlayerController 0)))
  (Default|ShowResult _asbp_main_pc true))

(event EventPostLogin
  (params (NewPlayer :type Player%20Controller%20Object%20Reference))
  ;[1 1 1] OnPostLogin
  ;;[1 1 1] PlayerState UID 세팅
  (bind _asbp_main_ps (Utilities|Casting|CastToBP_MainPS (Variables|/Script/Engine.Controller|GetPlayerState NewPlayer)))
  (Default|SetInfo _asbp_main_ps (Variables|Default|GetPlayerIndex))
  (bind _isoctopus (Default|SetRoleState _asbp_main_ps))
  (if _isoctopus
    (bind _returnvalue (CallFunction|GetInitialPosition NewPlayer))
    (bind _returnvalue_2 (Game|SpawnActorfromClass "/Game/Blueprints/Octopus/BP_VRPawnMain.BP_VRPawnMain_C" _returnvalue "AlwaysSpawn" 0 0))
    (Variables|/Game/Blueprints/Octopus/BP_VRPawnMain.BP_VRPawnMain_C|SetInitLoading _returnvalue_2 true)
    (Pawn|Possess NewPlayer _returnvalue_2)
    (Math|Integer|IncrementInt (Variables|Default|GetPlayerIndex))
    (else
      (bind _asbp_gi (Utilities|Casting|CastToBP_GI (Game|GetGameInstance)))
      (bind _returnvalue_3 (CallFunction|GetInitialPosition NewPlayer))
      (bind _returnvalue_4 (Game|SpawnActorfromClass (Variables|/Game/Blueprints/Public/BP_GI.BP_GI_C|GetDefaultHunterClass _asbp_gi) _returnvalue_3 "AlwaysSpawn" 0 0))
      (Pawn|Possess NewPlayer _returnvalue_4)
      (Math|Integer|IncrementInt (Variables|Default|GetPlayerIndex)))))

(fn ConstructionScript)

(fn GetHunterSpawnPoints
  (if (> (Utilities|Array|Length (Variables|Default|GetHunterRespawnPoints)) 0)
    _
    (else
      (bind _outactors (Actor|GetAllActorsOfClass "/Game/Blueprints/System/Main/BP_RespawnArea.BP_RespawnArea_C"))
      (Variables|Default|SetHunterRespawnPoints _outactors)))
  (Utilities|Array|Shuffle (Variables|Default|GetHunterRespawnPoints))
  (for _array_element (Variables|Default|GetHunterRespawnPoints)
    (bind _avaliable_ (Default|Avaliable _array_element))
    (if _avaliable_
      (bind _respawntransform (Default|GetRespawnPoint _array_element))
      (return _respawntransform)))
  ;[1 1 1] 모든 리스폰 포인트가 사용 불가능한 경우 - 맨 윗층에서 리스폰
  (bind _outactors_2 (Actor|GetAllActorswithTag "FinalSpawnPoint"))
  (bind _asbp_respawn_area (Utilities|Casting|CastToBP_RespawnArea (Utilities|Array|Get(acopy) _outactors_2 (Math|Random|RandomIntegerinRange 0 (- (Utilities|Array|Length _outactors_2) 1)))))
  (bind _respawntransform_2 (Default|GetRespawnPoint _asbp_respawn_area))
  (return _respawntransform_2))

(fn OnRepRemainRespawnNumber)

(fn GetInitialPosition
  (params (PlayerController :type Player%20Controller%20Object%20Reference))
  (bind _asbp_main_gs (Utilities|Casting|CastToBP_MainGS (Game|GetGameState)))
  (switch Utilities|FlowControl|Switch|SwitchonEMainGameState (Variables|/Game/Blueprints/System/Main/BP_MainGS.BP_MainGS_C|GetCurrentGameState _asbp_main_gs)
    (:NewEnumerator0
      (bind _outactors (Actor|GetAllActorswithTag "OctoLoading"))
      (return (Transformation|GetActorTransform (Utilities|Array|Get(acopy) _outactors))))
    (:NewEnumerator1
      (bind _asbp_main_ps (Utilities|Casting|CastToBP_MainPS (Variables|/Script/Engine.Controller|GetPlayerState PlayerController)))
      (if (Utilities|Enum|Equal(Enum) (Variables|/Game/Blueprints/System/Main/BP_MainPS.BP_MainPS_C|GetRoleState _asbp_main_ps) "NewEnumerator0")
        (bind _outactors_2 (Actor|GetAllActorswithTag "OctoStart"))
        (return (Transformation|GetActorTransform (Utilities|Array|Get(acopy) _outactors_2)))
        (else
          (bind _respawntransform (CallFunction|GetHunterSpawnPoints))
          (return _respawntransform))))))