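; Player state for the Octopus and Hunter roles, holding role and HP.
; On begin play it copies the role from the game instance and sets HP to that role's max.
; On the server, each tick below the game state's water height heals an Octopus or damages other roles, both through ApplyDamage, with healing as negative damage.
; HP functions clamp the value, and the CurrentHP RepNotify triggers the owning controller's widget update.
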(event Custom|DamageByWater
  (params (DeltaSeconds :type Float%20%28single-precision%29))
  ;[1 1 1] 헌터의 경우 물 데미지
  (bind _asbp_main_gs (Utilities|Casting|CastToBP_MainGS (Game|GetGameState)))
  (Game|Damage|ApplyDamage (Variables|Default|GetPawnPrivate) (* DeltaSeconds (Variables|/Game/Blueprints/System/Main/BP_MainGS.BP_MainGS_C|GetWaterDamage _asbp_main_gs)) 0 0))

(event Custom|HealingByWater
  (params (DeltaSeconds :type Float%20%28single-precision%29))
  ;[1 1 1] 문어의 경우 회복
  (bind _asbp_main_gs (Utilities|Casting|CastToBP_MainGS (Game|GetGameState)))
  (Game|Damage|ApplyDamage (Variables|Default|GetPawnPrivate) (* DeltaSeconds -1.0 (Variables|/Game/Blueprints/System/Main/BP_MainGS.BP_MainGS_C|GetWaterHealing _asbp_main_gs)) 0 0))

(event EventBeginPlay
  ;[1 1 1] Init
  (CallFunction|SetRoleState)
  (CallFunction|InitHP))

(event EventTick
  (params (DeltaSeconds :type Float%20%28single-precision%29))
  ;[1 1 1] Tick
  (Networking|SwitchHasAuthority
    (:Authority
      (Utilities|IsValid (Variables|Default|GetPawnPrivate)
        (:Is%20Valid
          (bind _asbp_main_gs (Utilities|Casting|CastToBP_MainGS (Game|GetGameState)))
          (if (> (Variables|/Game/Blueprints/System/Main/BP_MainGS.BP_MainGS_C|GetWaterHeight _asbp_main_gs) (.z (Transformation|GetActorLocation (Variables|Default|GetPawnPrivate))))
            (if (Utilities|Enum|Equal(Enum) (Variables|Default|GetRoleState) "NewEnumerator0")
              (CallFunction|HealingbyWater DeltaSeconds)
              (else
                (CallFunction|DamagebyWater DeltaSeconds)))))))))

(fn ConstructionScript)

(fn OnRepCurrentHP
  (bind _asbp_main_pc (Utilities|Casting|CastToBP_MainPC (Components|GetOwner)))
  (Utilities|IsValid _asbp_main_pc
    (:Is%20Valid
      (Default|UpdateHunterMainWidgetServer _asbp_main_pc))))

(fn InitHP
  (bind _maxhp (CallFunction|GetMaxHP))
  (Variables|Default|SetCurrentHP _maxhp))

(fn OnTakeDamage
  (params (Damage :type Float%20%28single-precision%29))
  (if (> (- (Variables|Default|GetCurrentHP) Damage) 0.0)
    (Variables|Default|SetCurrentHP (- (Variables|Default|GetCurrentHP) Damage))
    (else
      (Variables|Default|SetCurrentHP 0.0))))

(fn IsAlive
  (return (> (Variables|Default|GetCurrentHP) 0.0)))

(fn SetUID
  (params (UID :type Integer))
  (Variables|Default|SetUID UID))

(fn GetMaxHP
  (switch Utilities|FlowControl|Switch|SwitchonERoleState (Variables|Default|GetRoleState)
    (:NewEnumerator0
      (return (Variables|Default|GetOctoMaxHP)))
    (:NewEnumerator1
      (return (Variables|Default|GetHunterMaxHP)))))

(fn SetRoleState
  (bind _asbp_gi (Utilities|Casting|CastToBP_GI (Game|GetGameInstance)))
  (Utilities|IsValid _asbp_gi
    (:Is%20Valid
      (bind _output_get (Variables|Default|SetRoleState (Variables|/Game/Blueprints/Public/BP_GI.BP_GI_C|GetGI_RoleState _asbp_gi)))
      (Development|PrintString (Utilities|String|EnumtoString _output_get)))))

(fn OnHealingHP
  (params (Healing :type Float%20%28single-precision%29))
  (if (> (- (Variables|Default|GetCurrentHP) Healing) (Variables|Default|GetOctoMaxHP))
    (Variables|Default|SetCurrentHP (Variables|Default|GetOctoMaxHP))
    (else
      (Variables|Default|SetCurrentHP (- (Variables|Default|GetCurrentHP) Healing)))))