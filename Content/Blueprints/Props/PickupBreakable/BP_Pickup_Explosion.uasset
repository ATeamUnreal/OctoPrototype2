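; Breakable physics pickup prop that bursts with an explosion effect when it hits something hard after being dropped.
; On the authority, the Box hit event compares the impulse magnitude against a fixed threshold while IsDropped is set, then calls Destruction.
; Destruction stops Box physics and collision, hides the mesh and spawns the explosion emitter at the actor's transform, leaving the actor in the world without applying damage.
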(event OnComponentHit(Box)
  (params (HitComponent :type Primitive%20Component%20Object%20Reference) (OtherActor :type Actor%20Object%20Reference) (OtherComp :type Primitive%20Component%20Object%20Reference) (NormalImpulse :type Vector :default "0, 0, 0") (Hit :type Hit%20Result%20Structure%20%28by%20ref%29))
  ;[1 1 1] 일정 이상의 충격이 가해지면 부서짐
  (if (Variables|Default|GetIsDropped)
    (Networking|SwitchHasAuthority
      (:Authority
        (if (> (Math|Vector|VectorLength NormalImpulse) 7e+05)
          (CallFunction|Destruction))))))

(event Custom|Destruction
  (bind _returnvalue (Transformation|GetActorTransform))
  ;[1 1 1] 부서짐 효과
  (Physics|SetSimulatePhysics (Variables|Default|GetBox) false)
  (Collision|SetCollisionEnabled (Variables|Default|GetBox) "NoCollision")
  (Rendering|SetVisibility (Variables|Default|GetStaticMesh) false false)
  (Effects|SpawnEmitteratLocation (Variables|Default|GetExplosionEffect) (.location _returnvalue) (.rotation _returnvalue)))

(event EventBeginPlay
  (|CallParentFunction) ; 지금 이 노드는 비활성 상태입니다. \n핀을 끌어서 다른 노드를 연결하면 활성화됩니다.
)

(event Collision|EventActorBeginOverlap
  (params (OtherActor :type Actor%20Object%20Reference)))

(event EventTick
  (params (DeltaSeconds :type Float%20%28single-precision%29))
  (|CallParentFunction DeltaSeconds) ; 지금 이 노드는 비활성 상태입니다. \n핀을 끌어서 다른 노드를 연결하면 활성화됩니다.
)

(fn ConstructionScript
  (|CallParentFunction))