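; BP_Projectile_SN is a bullet projectile that flies without gravity and expires after BulletLife seconds.
; On any collision overlap it applies fixed damage credited to player controller 0 and spawns a scaled-up hit particle, without destroying itself.
; It then plays an impact sound at the collision location through a chain of events named for server-to-multicast relay.
; The BulletMove event is an empty stub.
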(event OnComponentBeginOverlap(BulletCollision)
  (params (OverlappedComponent :type Primitive%20Component%20Object%20Reference) (OtherActor :type Actor%20Object%20Reference) (OtherComp :type Primitive%20Component%20Object%20Reference) (OtherBodyIndex :type Integer) (bFromSweep :type Boolean) (SweepResult :type Hit%20Result%20Structure%20%28by%20ref%29))
  ;[1 1 1] Overlap
  (Game|Damage|ApplyDamage OtherActor 1e+01 (Game|GetPlayerController 0) self)
  (Effects|SpawnEmitteratLocation "/Game/Resources/Hunter/FX/Hits/P_Hit_Bullet.P_Hit_Bullet" (Transformation|GetWorldLocation (Variables|Default|GetBulletCollision)) "0, 0, 0" "10.000000,10.000000,10.000000")
  (CallFunction|PlayGunSound))

(event Custom|BulletMove
  ;[1 1 1] Bullet
)

(event Custom|MulticastGunSound
  (params (SoundLocation :type Vector))
  (Audio|SpawnSoundatLocation "/Game/Ultimate_SFX_Bundle/Warfare_SFX_Bundle/Bullet_Impacts_Flybys_Pro/Cues/Snow/Snow_6_Cue.Snow_6_Cue" SoundLocation "0, 0, 0" 1.0 1.0 0.0 0 0))

(event Custom|ServerGunSound
  (params (SoundLocation :type Vector))
  (CallFunction|MulticastGunSound SoundLocation))

(event Custom|PlayGunSound
  (CallFunction|ServerGunSound (Transformation|GetWorldLocation (Variables|Default|GetBulletCollision))))

(event EventBeginPlay
  ;[1 1 1] Bullet
  (Utilities|FlowControl|Sequence
    (:then_0
      (Variables|/Script/Engine.ProjectileMovementComponent|SetProjectileGravityScale (Variables|총알|GetProjectileMovement) 0.0)
      (Actor|SetLifeSpan (Variables|Default|GetBulletLife)))
    (:then_1
      (Variables|총알|SetProjectileMovement (Variables|총알|GetProjectileMovement)))))

(fn ConstructionScript)