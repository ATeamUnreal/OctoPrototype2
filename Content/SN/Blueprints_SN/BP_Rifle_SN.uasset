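; Rifle pickup actor that spins in place until an actor overlaps it.
; Tick applies a frame-rate-independent local rotation from WeaponRotateSpeed.
; On overlap it destroys itself before casting to BP_PlayerCharacter_SN, so any overlapping actor removes it.
; For the player, it calls WeaponAttachment unless PickupWeapon already equals one specific enum value.
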(event EventTick
  (params (DeltaSeconds :type Float%20%28single-precision%29))
  ;[1 1 1] WeaponRotation
  (Transformation|AddActorLocalRotation (* (Variables|Default|GetWeaponRotateSpeed) (Utilities|Time|GetWorldDeltaSeconds)) false false))

(event Collision|EventActorBeginOverlap
  (params (OtherActor :type Actor%20Object%20Reference))
  (Actor|DestroyActor)
  (bind _asbp_player_character_sn (Utilities|Casting|CastToBP_PlayerCharacter_SN OtherActor))
  (if (not (Utilities|Enum|Equal(Enum) (Variables|/Game/SN/Blueprints_SN/BP_PlayerCharacter_SN.BP_PlayerCharacter_SN_C|GetPickupWeapon _asbp_player_character_sn) "NewEnumerator3"))
    (Default|WeaponAttachment _asbp_player_character_sn)))

(fn ConstructionScript)