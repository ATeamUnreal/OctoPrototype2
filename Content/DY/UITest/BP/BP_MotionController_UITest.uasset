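; Test VR motion controller actor that detects when a hand points at UI and sizes that hand's laser.
; Each tick it line-traces a short distance forward from the controller against one object type.
; A hit tells the VR pawn to attach UI use to this hand and stretches the Ray to the hit point; a miss releases it.
; The Ray starts hidden and is never shown in this Blueprint.
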(event EventTick
  (params (DeltaSeconds :type Float%20%28single-precision%29))
  (bind _motioncontroller (Variables|Default|GetMotionController))
  (bind _returnvalue (Transformation|GetWorldLocation _motioncontroller))
  ;[1 1 1] UI체크를 위한 LineTrace
  (bind (_outhit _returnvalue_2) (Collision|LineTraceForObjects _returnvalue (+ _returnvalue (* (Math|Vector|GetForwardVector _motioncontroller) 2e+02)) (Utilities|Array|MakeArray "ObjectTypeQuery7") false 0 "None"))
  (if _returnvalue_2
    ;[1 1 1] 폰에게 이 손이 UI를 사용한다고 알림
    (Default|UIHandAttach (Variables|Default|GetVRPawn) self)
    (CallFunction|RayVisualUpdate _outhit)
    (else
      ;[1 1 1] UI 인터렉션 비활성화
      (Default|UIHandRelease (Variables|Default|GetVRPawn) self))))

(event EventBeginPlay
  ;[1 1 1] 코멘트
  (bind _asbp_vrpawn_uitest (Utilities|Casting|CastToBP_VRPawn_UITest (Game|Player|GetPlayerPawn 0)))
  (Variables|Default|SetVRPawn _asbp_vrpawn_uitest)
  (Rendering|SetVisibility (Variables|Default|GetRay) false false))

(fn ConstructionScript)

(fn RayVisualUpdate
  (params (Hit :type Hit%20Result%20Structure%20%28by%20ref%29))
  (bind _location (Collision|BreakHitResult Hit))
  (bind _motioncontroller (Variables|Default|GetMotionController))
  (bind _returnvalue (Transformation|GetWorldLocation _motioncontroller))
  (bind _returnvalue_2 (Math|Vector|Distance(Vector) _location _returnvalue))
  ;[1 1 1] UI 레이저 모델 업데이트
  (Transformation|SetRelativeScale3D (Variables|Default|GetRay) (Math|Vector|MakeVector _returnvalue_2 1.0 1.0))
  (Transformation|SetRelativeLocation (Variables|Default|GetRay) (Math|Vector|MakeVector (/ _returnvalue_2 2.0) 0.0 0.0) false false))